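; Player character for a shooter-style item hunt, with camera-relative movement, bullet firing and a jump that adds a forward impulse at high speed.
; BeginPlay rolls a random key item from color, type and size tables, builds a "Find a…" objective phrase, and resets camera rotation.
; Shooting also prints the objective in its color.
; A reroll event spawns objects, using weighted random rolls for the key-item flag and key-or-random appearance.
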(event Custom|Roll_KeyItem
  ;[1 1 1] Rolls key item randomly
  (Variables|Default|SetKeyItem (Utilities|Struct|MakeItemStruct (Math|Random|RandomIntegerinRange 0 (- (Utilities|Array|Length (Variables|Default|GetColors)) 1)) (Math|Random|RandomIntegerinRange 0 (- (Utilities|Array|Length (Variables|Default|GetTypes)) 1)) (Math|Random|RandomIntegerinRange 0 (- (Utilities|Array|Length (Variables|Default|GetExtraModifiers)) 1)))))

(event Custom|Clean_KeyItem
  (Variables|Default|SetKeyItem (Utilities|Struct|MakeItemStruct 0 0 0)))

(event Custom|RerollRandomObjectOrKey
  (params (PositionToSpawn :type Vector))
  (bind _spawnratemin (Variables|Default|GetSpawnRateMin))
  (bind _extramodifiers (Variables|Default|GetExtraModifiers))
  (bind _extramodifiers_2 (Variables|Default|GetExtraModifiers))
  (bind _keyitem (Variables|Default|GetKeyItem))
  (bind _extramodifiers_3 (Variables|Default|GetExtraModifiers))
  (bind _spawnratemax (Variables|Default|GetSpawnRateMax))
  (bind _returnvalue (Utilities|Array|Length _extramodifiers_2))
  (bind _returnvalue_2 (Math|Random|RandomFloatinRange _spawnratemin _spawnratemax))
  (bind _output (Utilities|Array|Get(acopy) _extramodifiers_3 (.extramodifier _keyitem)))
  (bind _returnvalue_3 (Math|Random|RandomBoolwithWeight _returnvalue_2))
  (bind _returnvalue_4 (- _returnvalue 1))
  (bind _returnvalue_5 (Math|Random|RandomIntegerinRange 0 _returnvalue_4))
  (bind _output_2 (Utilities|Array|Get(acopy) _extramodifiers _returnvalue_5))
  ;[1 1 1] Get Random item or key item based on SpawnRatemin and SpawnRateMax
  (bind _returnvalue_6 (Game|SpawnActorfromClass "/Game/Blueprints/Objects.Objects_C" (Math|Transform|MakeTransform (+ PositionToSpawn "0, 0,15.000000") "0, 0, 0" "1,1,1") "Undefined" 0 0))
  (Variables|/Game/Blueprints/Objects.Objects_C|SetAmIKeyItem? _returnvalue_6 _returnvalue_3)
  (Variables|/Game/Blueprints/Objects.Objects_C|SetConstructor _returnvalue_6 (select _returnvalue_3 (Utilities|Struct|MakeObjectBuildStruct (.color (Utilities|Array|Get(acopy) (Variables|Default|GetColors) (.color _keyitem))) (.type (Utilities|Array|Get(acopy) (Variables|Default|GetTypes) (.type _keyitem))) (.min_size _output) (.max_size _output)) (Utilities|Struct|MakeObjectBuildStruct (.color (Utilities|Array|Get(acopy) (Variables|Default|GetColors) (Math|Random|RandomIntegerinRange 0 (- (Utilities|Array|Length (Variables|Default|GetColors)) 1)))) (.type (Utilities|Array|Get(acopy) (Variables|Default|GetTypes) (Math|Random|RandomIntegerinRange 0 (- (Utilities|Array|Length (Variables|Default|GetTypes)) 1)))) (.min_size _output_2) (.max_size _output_2)))))

(event EventBeginPlay
  (bind _colors (Variables|Default|GetColors))
  (bind _keyitem (Variables|Default|GetKeyItem))
  (bind _output (Utilities|Array|Get(acopy) _colors (.color _keyitem)))
  ;[1 1 1] BeginPlay
  (Utilities|FlowControl|Sequence
    (:then_0
      (CallFunction|RollKeyItem)
      ;[1 1 1] Create phrase and objective color
      (bind _output_get (Variables|Default|SetPhrase (Utilities|String|Append "Find a " (.size (Utilities|Array|Get(acopy) (Variables|Default|GetExtraModifiers) (.extramodifier _keyitem))) " " (.name _output) " " (.name (Utilities|Array|Get(acopy) (Variables|Default|GetTypes) (.type _keyitem))) ".")))
      (Variables|Default|SetColor (.color _output))
      (Development|PrintString _output_get))
    (:then_1
      ;[1 1 1] Camera reset on Load/Reset Save
      (Pawn|SetControlRotation (Game|GetPlayerController 0) (Transformation|GetActorRotation)))))

(event Input|ActionEvents|InputActionJump
  (params (Key :type Key%20Structure :default "None"))
  (bind _returnvalue (Transformation|GetVelocity))
  (bind _charactermovement (Variables|Character|GetCharacterMovement))
  (bind _maxwalkspeed (Variables|/Script/Engine.CharacterMovementComponent|GetMaxWalkSpeed _charactermovement))
  ;[1 1 1] Jump (Jumps higher and gives an impulse if player is at max speed)
  (:Pressed
    (if (or (> (Math|Float|Absolute(Float) (.x _returnvalue)) _maxwalkspeed) (> (Math|Float|Absolute(Float) (.y _returnvalue)) _maxwalkspeed))
      (Physics|AddImpulse (Variables|/Script/Engine.MovementComponent|GetUpdatedPrimitive (Variables|Character|GetCharacterMovement)) (Math|Vector|GetForwardVector (Math|Rotator|MakeRotator 0.0 0.0 (.Yaw (Math|Rotator|BreakRotator (Class|SpringArmComponent|GetTargetRotation (Variables|Default|GetSpringArm)))))) "None" false))
    (Character|Jump))
  (:Released
    (Character|StopJumping)))

(event Input|ActionEvents|InputActionShoot
  (params (Key :type Key%20Structure :default "None"))
  ;[1 1 1] Shoots
  (:Pressed
    (Game|SpawnActorfromClass "/Game/Blueprints/Bullet.Bullet_C" (Transformation|GetWorldTransform (Variables|Default|GetBulletSpawnPoint)) "Undefined" 0 0)
    (Development|PrintString (Variables|Default|GetPhrase) true true (Variables|Default|GetColor) 21312312.0)))

(event Input|AxisEvents|InputAxisMoveLeftRight
  (params (AxisValue :type Float%20%28single-precision%29))
  ;[1 1 1] Walks based on camera orientation
  (Pawn|Input|AddMovementInput (Math|Vector|GetRightVector (Math|Rotator|MakeRotator 0.0 0.0 (.Yaw (Math|Rotator|BreakRotator (Class|SpringArmComponent|GetTargetRotation (Variables|Default|GetSpringArm)))))) AxisValue false))

(event Input|AxisEvents|InputAxisMoveUpDown
  (params (AxisValue :type Float%20%28single-precision%29))
  ;[1 1 1] Walks based on camera orientation
  (Pawn|Input|AddMovementInput (Math|Vector|GetForwardVector (Math|Rotator|MakeRotator 0.0 0.0 (.Yaw (Math|Rotator|BreakRotator (Class|SpringArmComponent|GetTargetRotation (Variables|Default|GetSpringArm)))))) AxisValue false))

(fn ConstructionScript)

(fn GeneratePhrase
  (bind _colors (Variables|Default|GetColors))
  (bind _keyitem (Variables|Default|GetKeyItem))
  (bind _output (Utilities|Array|Get(acopy) _colors (.color _keyitem)))
  ;[1 1 1] Creates the phrase and shows the key object color
  (Variables|Default|SetPhrase (Utilities|String|Append "Find a " (.size (Utilities|Array|Get(acopy) (Variables|Default|GetExtraModifiers) (.extramodifier _keyitem))) " " (.name _output) " " (.name (Utilities|Array|Get(acopy) (Variables|Default|GetTypes) (.type _keyitem))) "."))
  (Variables|Default|SetColor (.color _output))
  (return "" ""))