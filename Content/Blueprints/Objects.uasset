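; Spawnable object that sets up its look from a Constructor struct and flags whether it is the key item.
; After a brief delay, it compares KeyItem and MyItem by color, type and modifier.
; It applies a colored dynamic material, the given mesh or a random cloud mesh for cloud types, and a random uniform scale within range.
; Non-key objects destroy themselves after a timeout.
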(event EventBeginPlay
  (bind _object (Variables|Default|GetObject))
  (bind _object_2 (Variables|Default|GetObject))
  (bind _constructor (Variables|Default|GetConstructor))
  (bind _keyitem (Variables|Default|GetKeyItem))
  (bind _myitem (Variables|Default|GetMyItem))
  (Utilities|FlowControl|Delay 0.1)
  ;[1 1 1] Set Parameters based on random roll from character
  (Variables|Default|SetAmIKeyItem? (and (and (== (.color _keyitem) (.color _myitem)) (== (.type _keyitem) (.type _myitem))) (== (.extramodifier _keyitem) (.extramodifier _myitem))))
  (if (== (.type (Variables|Default|GetConstructor)) "/Game/Meshes/Obstacles/Cloud_01.Cloud_01")
    (bind _returnvalue (Rendering|Material|CreateDynamicMaterialInstance _object 0 "/Game/Materials/Mesh_Materials/Dream/M_Dream_Cloud.M_Dream_Cloud" "None" :!class /Script/Engine.PrimitiveComponent))
    (Rendering|Material|SetMaterial _object 0 _returnvalue)
    (Rendering|Material|SetVectorParameterValue _returnvalue "FinalColor" (.color _constructor) :!class /Script/Engine.MaterialInstanceDynamic)
    (Components|StaticMesh|SetStaticMesh _object_2 (.OutItem (Utilities|Array|Random (Variables|Default|GetClouds))))
    (else
      (bind _returnvalue_2 (Rendering|Material|CreateDynamicMaterialInstance _object 0 "/Game/Materials/Colors/Color.Color" "None" :!class /Script/Engine.PrimitiveComponent))
      (Rendering|Material|SetMaterial _object 0 _returnvalue_2)
      (Rendering|Material|SetVectorParameterValue _returnvalue_2 "FinalColor" (.color _constructor) :!class /Script/Engine.MaterialInstanceDynamic)
      (Components|StaticMesh|SetStaticMesh _object (.type _constructor))))
  (Transformation|SetRelativeScale3D _object_2 (* "1.000000,1.000000,1.000000" (Math|Random|RandomFloatinRange (.min_size _constructor) (.max_size _constructor))))
  ;[1 1 1] Destroy in 30 seconds if not key item
  (if (not (Variables|Default|GetAmIKeyItem?))
    (Utilities|FlowControl|Delay 3e+01)
    (Actor|DestroyActor)))

(fn ConstructionScript)