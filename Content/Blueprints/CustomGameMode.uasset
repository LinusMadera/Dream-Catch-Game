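; Game mode that tracks the score and high score and handles level flow.
; BeginPlay loads AllTimeBest from the "Save2" slot, or creates that save if missing.
; Next increments CurrentScore and opens "Normal"; EraseScore resets it.
; Over writes CurrentScore as HighScore without comparing it to the stored best, resets the score and opens "EndMap".
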(event Custom|EraseScore
  (Variables|Default|SetCurrentScore 0))

(event Custom|Save%20Game
  ;[1 1 1] Saving game
  (bind _returnvalue (SaveGame|LoadGamefromSlot "Save2"))
  (bind _asbp_save_game_variables (Utilities|Casting|CastToBP_SaveGame_Variables _returnvalue))
  (Variables|/Game/Blueprints/SaveGame/BP_SaveGame_Variables.BP_SaveGame_Variables_C|SetHigh%20Score _asbp_save_game_variables (Variables|Default|GetCurrentScore))
  (SaveGame|SaveGametoSlot _asbp_save_game_variables "Save2"))

(event Custom|Over
  (CallFunction|SaveGame)
  (Variables|Default|SetCurrentScore 0)
  (Game|OpenLevel(byName) "EndMap"))

(event Custom|Next
  (Math|Integer|IncrementInt (Variables|Default|GetCurrentScore)
    (:%20%20
      (Game|OpenLevel(byName) "Normal"))))

(event EventBeginPlay
  (bind _returnvalue (SaveGame|DoesSaveGameExist "Save2"))
  (if _returnvalue
    ;[1 1 1] Loading Game
    (bind _returnvalue_2 (SaveGame|LoadGamefromSlot "Save2"))
    (bind _asbp_save_game_variables (Utilities|Casting|CastToBP_SaveGame_Variables _returnvalue_2))
    (Variables|Default|SetAllTimeBest (Variables|/Game/Blueprints/SaveGame/BP_SaveGame_Variables.BP_SaveGame_Variables_C|GetHigh%20Score _asbp_save_game_variables))
    (else
      ;[1 1 1] Creating a save file - To delete this file go to, project file, Saved, SaveGames, Delete the save file
      (bind _returnvalue_3 (SaveGame|CreateSaveGameObject "/Game/Blueprints/SaveGame/BP_SaveGame_Variables.BP_SaveGame_Variables_C"))
      (SaveGame|SaveGametoSlot _returnvalue_3 "Save2"))))

(fn ConstructionScript)