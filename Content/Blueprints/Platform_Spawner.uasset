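; Platform spawner actor that builds a randomized square grid of floor tiles when play begins.
; Each cell usually gets a plain instanced static mesh tile plus a Platforms_ObjectSpawner actor at the same location.
; Occasionally it instead gets a random one of three hole-tile instanced meshes, rotated in random quarter turns, with no object spawner.
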(event EventBeginPlay
  (Variables|Default|SetHoleTiles (Utilities|Array|MakeArray (Variables|Default|GetHole0) (Variables|Default|GetHole1) (Variables|Default|GetHole2)))
  (for _index (range 0 50)
    (for _index_2 (range 0 50)
      (Variables|Default|SetSpawnX (* _index_2 6e+02))
      (Variables|Default|SetSpawnY (* _index 6e+02))
      (if (< 3 (Math|Random|RandomIntegerinRange 0 29))
        (Components|InstancedStaticMesh|AddInstance (Variables|Default|GetInstancedStaticMesh) (Math|Transform|MakeTransform (Math|Vector|MakeVector (Variables|Default|GetSpawnX) (Variables|Default|GetSpawnY) 0.0) "0, 0, 0" "1,1,1"))
        (Game|SpawnActorfromClass "/Game/Blueprints/Platforms_ObjectSpawner.Platforms_ObjectSpawner_C" (Math|Transform|MakeTransform (Math|Vector|MakeVector (Variables|Default|GetSpawnX) (Variables|Default|GetSpawnY) 0.0) "0, 0, 0" "1,1,1") "Undefined" 0 0)
        (else
          (Components|InstancedStaticMesh|AddInstance (.OutItem (Utilities|Array|Random (Variables|Default|GetHoleTiles))) (Math|Transform|MakeTransform (Math|Vector|MakeVector (Variables|Default|GetSpawnX) (Variables|Default|GetSpawnY) 0.0) (Math|Rotator|MakeRotator 0.0 0.0 (* (Math|Random|RandomIntegerinRange 0 3) 9e+01)) "1,1,1")))))))

(fn ConstructionScript)